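; Behavior tree task that picks the guard enemy's current patrol point for its AI.
; It casts the controlled pawn to Guard_Enemy_AI, then writes a random navigable location near the current PatrolPath actor to a blackboard vector.
; It also sets a blackboard wait time randomized by that point's WaitTime and WaitDeviation, then finishes successfully.
; The path index is only read here, and a failed cast never finishes the task.
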(event EventReceiveExecuteAI
  (params (OwnerController :type AI%20Controller%20Object%20Reference) (ControlledPawn :type Pawn%20Object%20Reference))
  (bind _asguard_enemy_ai (Utilities|Casting|CastToGuard_Enemy_AI ControlledPawn))
  (bind _output_get (Variables|Default|SetGuard%20Enemy%20Pawn _asguard_enemy_ai))
  (AI|BehaviorTree|SetBlackboardValueasVector (Variables|Default|GetBB_TargetVector) (.RandomLocation (Class|NavigationSystemV1|GetRandomPointinNavigableRadius (Transformation|GetActorLocation (Utilities|Array|Get(acopy) (Variables|/Game/Blueprints/Enemy/Guard_Enemy_AI.Guard_Enemy_AI_C|GetPatrolPath _output_get) (Variables|/Game/Blueprints/Enemy/Guard_Enemy_AI.Guard_Enemy_AI_C|GetCurrentPathIndex _output_get))) 2e+01 0 0)))
  (Class|BTFunctionLibrary|SetBlackboardValueasFloat (Variables|Default|GetBB_WaitTime) (Math|Random|RandomFloatinRange (- (Variables|/Game/Blueprints/Enemy/PathPoint.PathPoint_C|GetWaitTime (Utilities|Array|Get(acopy) (Variables|/Game/Blueprints/Enemy/Guard_Enemy_AI.Guard_Enemy_AI_C|GetPatrolPath (Variables|Default|GetGuard%20Enemy%20Pawn)) (Variables|/Game/Blueprints/Enemy/Guard_Enemy_AI.Guard_Enemy_AI_C|GetCurrentPathIndex (Variables|Default|GetGuard%20Enemy%20Pawn)))) (Variables|/Game/Blueprints/Enemy/PathPoint.PathPoint_C|GetWaitDeviation (Utilities|Array|Get(acopy) (Variables|/Game/Blueprints/Enemy/Guard_Enemy_AI.Guard_Enemy_AI_C|GetPatrolPath (Variables|Default|GetGuard%20Enemy%20Pawn)) (Variables|/Game/Blueprints/Enemy/Guard_Enemy_AI.Guard_Enemy_AI_C|GetCurrentPathIndex (Variables|Default|GetGuard%20Enemy%20Pawn))))) (+ (Variables|/Game/Blueprints/Enemy/PathPoint.PathPoint_C|GetWaitTime (Utilities|Array|Get(acopy) (Variables|/Game/Blueprints/Enemy/Guard_Enemy_AI.Guard_Enemy_AI_C|GetPatrolPath (Variables|Default|GetGuard%20Enemy%20Pawn)) (Variables|/Game/Blueprints/Enemy/Guard_Enemy_AI.Guard_Enemy_AI_C|GetCurrentPathIndex (Variables|Default|GetGuard%20Enemy%20Pawn)))) (Variables|/Game/Blueprints/Enemy/PathPoint.PathPoint_C|GetWaitDeviation (Utilities|Array|Get(acopy) (Variables|/Game/Blueprints/Enemy/Guard_Enemy_AI.Guard_Enemy_AI_C|GetPatrolPath (Variables|Default|GetGuard%20Enemy%20Pawn)) (Variables|/Game/Blueprints/Enemy/Guard_Enemy_AI.Guard_Enemy_AI_C|GetCurrentPathIndex (Variables|Default|GetGuard%20Enemy%20Pawn)))))))
  (AI|BehaviorTree|FinishExecute true))