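; Pipe trigger that spills lava when shot and damages the first-person player standing in it.
; When an end overlap leaves no projectile in Box, it unhides the magma flow and spill, disables Box collision, then hides both after LavaDisperseTime.
; Entering Lava while the flow is visible starts a half-second damage loop that repeats while the player overlaps the actor, without rechecking visibility.
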(event OnComponentEndOverlap(Box)
  (params (OverlappedComponent :type Primitive%20Component%20Object%20Reference) (OtherActor :type Actor%20Object%20Reference) (OtherComp :type Primitive%20Component%20Object%20Reference) (OtherBodyIndex :type Integer))
  ;[1 1 1] Spawn Lava when shot
  (Utilities|IsValid (Utilities|Array|Get(acopy) (Collision|GetOverlappingActors (Variables|Default|GetBox) "/Game/Blueprints/FirstPersonTemplate/BP_FirstPersonProjectile.BP_FirstPersonProjectile_C" :!class /Script/Engine.PrimitiveComponent))
    (:Is%20Not%20Valid
      (Development|PrintString "LavaSpawn(Animation Here)")
      (Development|SetHiddeninGame (Variables|Default|GetSM_Env_Fire_Magma01_smallFlow) false false)
      (Collision|SetCollisionEnabled (Variables|Default|GetBox) "NoCollision")
      ;[1 1 1] Hide Lava after timer
      (Utilities|FlowControl|Delay (Variables|Default|GetLava%20Disperse%20Time))
      (if (Rendering|IsVisible (Variables|Default|GetSM_Env_Fire_Magma01_smallFlow))
        (Development|SetHiddeninGame (Variables|Default|GetSM_Env_Fire_Magma01_smallFlow) true false)
        (if (Rendering|IsVisible (Variables|Default|GetLavaSpill))
          (Development|SetHiddeninGame (Variables|Default|GetLavaSpill) true false))))))

(event OnComponentBeginOverlap(Lava)
  (params (OverlappedComponent :type Primitive%20Component%20Object%20Reference) (OtherActor :type Actor%20Object%20Reference) (OtherComp :type Primitive%20Component%20Object%20Reference) (OtherBodyIndex :type Integer) (bFromSweep :type Boolean) (SweepResult :type Hit%20Result%20Structure%20%28by%20ref%29))
  ;[1 1 1] TakeLavaDamage
  (Utilities|IsValid (Utilities|Array|Get(acopy) (Collision|GetOverlappingActors (Variables|Default|GetLava) "/Game/Blueprints/FirstPersonTemplate/BP_FirstPersonCharacter.BP_FirstPersonCharacter_C" :!class /Script/Engine.PrimitiveComponent))
    (:Is%20Valid
      (if (Rendering|IsVisible (Variables|Default|GetSM_Env_Fire_Magma01_smallFlow))
        (Development|PrintString "InLava")
        (bind _asbp_first_person_character (Utilities|Casting|CastToBP_FirstPersonCharacter OtherActor)
          (:then
            (bind _output_get (Variables|Default|SetPlayerCharacter _asbp_first_person_character))
            (Default|TakeDamage _output_get :!label _label)
            (Utilities|FlowControl|Delay 0.5)
            (if (Collision|IsOverlappingActor (Variables|Default|GetPlayerCharacter) :!class /Script/Engine.Actor)
              (goto _label)))
          (:CastFailed
            (Development|PrintString "CastFailed")))
        (else
          (Development|PrintString "NoLavaSpawn"))))))

(fn ConstructionScript)