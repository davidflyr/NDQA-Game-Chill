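; Health pickup that heals the first-person character when it overlaps the pickup's box while below full health.
; The overlap event confirms an overlapping BP_FirstPersonCharacter, reads its health and calls HealDamage on it if under the cap.
; Once used, the pickup disables box and mesh collision and hides the mesh instead of destroying itself.
; Debug strings report healing, full health or a failed cast.
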(event OnComponentBeginOverlap(Box)
  (params (OverlappedComponent :type Primitive%20Component%20Object%20Reference) (OtherActor :type Actor%20Object%20Reference) (OtherComp :type Primitive%20Component%20Object%20Reference) (OtherBodyIndex :type Integer) (bFromSweep :type Boolean) (SweepResult :type Hit%20Result%20Structure%20%28by%20ref%29))
  (Utilities|IsValid (Utilities|Array|Get(acopy) (Collision|GetOverlappingActors (Variables|Default|GetBox) "/Game/Blueprints/FirstPersonTemplate/BP_FirstPersonCharacter.BP_FirstPersonCharacter_C" :!class /Script/Engine.PrimitiveComponent))
    (:Is%20Valid
      (bind _asbp_first_person_character (Utilities|Casting|CastToBP_FirstPersonCharacter OtherActor))
      (bind _currenthealth (Default|GetHealth _asbp_first_person_character))
      (if (< _currenthealth 1e+02)
        (Development|PrintString "Healing")
        (bind _asbp_first_person_character_2 (Utilities|Casting|CastToBP_FirstPersonCharacter OtherActor)
          (:then
            (bind _output_get (Variables|Default|SetPlayerCharacter _asbp_first_person_character_2))
            (Default|HealDamage _output_get)
            (Collision|SetCollisionEnabled (Variables|Default|GetBox) "NoCollision")
            (Development|SetHiddeninGame (Variables|Debug|GetStaticMeshComponent) true false)
            (Collision|SetCollisionEnabled (Variables|Debug|GetStaticMeshComponent) "NoCollision"))
          (:CastFailed
            (Development|PrintString "Cast Failed")))
        (else
          (Development|PrintString "Full Health"))))))

(fn ConstructionScript)