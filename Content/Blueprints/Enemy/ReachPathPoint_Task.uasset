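; Behavior tree task that advances a Guard_Enemy_AI pawn to the next index on its PatrolPath, finishing as failed.
; At the path's end, PatrolPathBehavior decides: Do Nothing finishes as success, and Loop resets the index to zero and succeeds.
; Patrol Back sets PathDirection to -1 and fails, though this task never reads that direction and only steps the index forward.
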(event EventReceiveExecuteAI
  (params (OwnerController :type AI%20Controller%20Object%20Reference) (ControlledPawn :type Pawn%20Object%20Reference))
  (bind _asguard_enemy_ai (Utilities|Casting|CastToGuard_Enemy_AI ControlledPawn))
  (bind _output_get (Variables|Default|SetGuardEnemyPawn _asguard_enemy_ai))
  (if (Utilities|Array|IsValidIndex (Variables|/Game/Blueprints/Enemy/Guard_Enemy_AI.Guard_Enemy_AI_C|GetPatrolPath _output_get) (+ (Variables|/Game/Blueprints/Enemy/Guard_Enemy_AI.Guard_Enemy_AI_C|GetCurrentPathIndex _output_get) 1))
    (Variables|/Game/Blueprints/Enemy/Guard_Enemy_AI.Guard_Enemy_AI_C|SetCurrentPathIndex (Variables|Default|GetGuardEnemyPawn) (+ (Variables|/Game/Blueprints/Enemy/Guard_Enemy_AI.Guard_Enemy_AI_C|GetCurrentPathIndex (Variables|Default|GetGuardEnemyPawn)) 1))
    (AI|BehaviorTree|FinishExecute false)
    (else
      (switch Utilities|FlowControl|Switch|SwitchonPatrolPathEnding (Variables|/Game/Blueprints/Enemy/Guard_Enemy_AI.Guard_Enemy_AI_C|GetPatrol%20Path%20Behavior (Variables|Default|GetGuardEnemyPawn))
        (:NewEnumerator0
          (AI|BehaviorTree|FinishExecute true))
        (:NewEnumerator1
          (Variables|/Game/Blueprints/Enemy/Guard_Enemy_AI.Guard_Enemy_AI_C|SetPathDirection (Variables|Default|GetGuardEnemyPawn) -1)
          (AI|BehaviorTree|FinishExecute false))
        (:NewEnumerator2
          (Variables|/Game/Blueprints/Enemy/Guard_Enemy_AI.Guard_Enemy_AI_C|SetCurrentPathIndex (Variables|Default|GetGuardEnemyPawn) 0)
          (AI|BehaviorTree|FinishExecute true))))))