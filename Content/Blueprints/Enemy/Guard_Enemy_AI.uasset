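; Guard enemy character that hurts the first-person player on contact and is destroyed when its health runs out.
; Capsule overlap damages the player repeatedly while contact lasts; end overlap applies self-damage if a projectile is still overlapping.
; BeginPlay sets walk speed.
; Random wander and perception-to-AI-controller target updates are disconnected, leaving TargetLost's key-clearing without an active timer.
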(event OnTargetPerceptionUpdated(AIPerception)
  (params (Actor :type Actor%20Object%20Reference) (Stimulus :type AI%20Stimulus%20Structure))
  ;[1 1 1] Behavior
)

(event OnComponentBeginOverlap(CapsuleComponent)
  (params (OverlappedComponent :type Primitive%20Component%20Object%20Reference) (OtherActor :type Actor%20Object%20Reference) (OtherComp :type Primitive%20Component%20Object%20Reference) (OtherBodyIndex :type Integer) (bFromSweep :type Boolean) (SweepResult :type Hit%20Result%20Structure%20%28by%20ref%29))
  ;[1 1 1] DamagePlayer
  (Utilities|IsValid (Utilities|Array|Get(acopy) (Collision|GetOverlappingActors (Variables|Collision|GetCapsuleComponent) "/Game/Blueprints/FirstPersonTemplate/BP_FirstPersonCharacter.BP_FirstPersonCharacter_C" :!class /Script/Engine.PrimitiveComponent))
    (:Is%20Valid
      (bind _asbp_first_person_character (Utilities|Casting|CastToBP_FirstPersonCharacter OtherActor)
        (:then
          (bind _output_get (Variables|Default|SetPlayerCharacter _asbp_first_person_character))
          (Default|TakeDamage _output_get :!label _label)
          (Utilities|FlowControl|Delay 2.0)
          (if (Collision|IsOverlappingActor (Variables|Default|GetPlayerCharacter) :!class /Script/Engine.Actor)
            (goto _label)))
        (:CastFailed
          (Development|PrintString "CastFailed"))))))

(event OnComponentEndOverlap(CapsuleComponent)
  (params (OverlappedComponent :type Primitive%20Component%20Object%20Reference) (OtherActor :type Actor%20Object%20Reference) (OtherComp :type Primitive%20Component%20Object%20Reference) (OtherBodyIndex :type Integer))
  ;[1 1 1] DamageEnemy
  (Utilities|IsValid (Utilities|Array|Get(acopy) (Collision|GetOverlappingActors (Variables|Collision|GetCapsuleComponent) "/Game/Blueprints/FirstPersonTemplate/BP_FirstPersonProjectile.BP_FirstPersonProjectile_C" :!class /Script/Engine.PrimitiveComponent))
    (:Is%20Valid
      (CallFunction|TakeDamage))))

(event Custom|RandomWander
  ;[1 1 1] Simple Wander
)

(event Custom|TargetLost
  ;[1 1 1] Behavior
  (Variables|Default|SetPerceivedActor 0)
  (Default|UpdateTargetActorKey (.AsAIC%20Third%20Person%20Character (Utilities|Casting|CastToAIC_ThirdPersonCharacter (Pawn|GetController)))))

(event EventBeginPlay
  ;[1 1 1] WalkSpeed
  (Variables|/Script/Engine.CharacterMovementComponent|SetMaxWalkSpeed (Variables|Character|GetCharacterMovement) (Variables|Default|GetMaxWalkSpeed)))

(fn ConstructionScript)

(fn TakeDamage
  (bind _output_get (Variables|Default|SetHealth (- (Variables|Default|GetHealth) (Variables|Default|GetDamage%20Taken))))
  (if (<= _output_get 0.5)
    (Actor|DestroyActor)))