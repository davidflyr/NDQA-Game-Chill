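; Destructible wall actor that releases a waterfall and leaves standing water that slows the player.
; When a Box overlap ends with no projectile left inside, it reveals water and flow meshes, disables the Box collision and plays a steam sound.
; After WaterDisperseTime the sound stops and the flows hide, leaving the water planes visible.
; The WaterSlow volume calls the character's slow on entry if water is visible, and reverses it on exit.
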(event OnComponentEndOverlap(Box)
  (params (OverlappedComponent :type Primitive%20Component%20Object%20Reference) (OtherActor :type Actor%20Object%20Reference) (OtherComp :type Primitive%20Component%20Object%20Reference) (OtherBodyIndex :type Integer))
  ;[1 1 1] OnTriggerStartWaterFall
  (Utilities|IsValid (Utilities|Array|Get(acopy) (Collision|GetOverlappingActors (Variables|Default|GetBox) "/Game/Blueprints/FirstPersonTemplate/BP_FirstPersonProjectile.BP_FirstPersonProjectile_C" :!class /Script/Engine.PrimitiveComponent))
    (:Is%20Not%20Valid
      (Development|PrintString "SpawnWaterAnimation")
      (Development|SetHiddeninGame (Variables|Default|GetSM_WaterPlain1) false false)
      ;[1 1 1] HideWaterFall&StopSound
      (Collision|SetCollisionEnabled (Variables|Default|GetBox) "NoCollision")
      (bind _returnvalue (Audio|SpawnSound2D "/Game/StarterContent/Audio/Steam01.Steam01" 1.0 1.0 0.0 0))
      (Utilities|FlowControl|Delay (Variables|Default|GetWater%20Disperse%20Time))
      (Audio|Components|Audio|Stop _returnvalue)
      (Development|SetHiddeninGame (Variables|Default|GetSM_Env_Fire_Magma01_smallFlow) true false))))

(event OnComponentEndOverlap(WaterSlow)
  (params (OverlappedComponent :type Primitive%20Component%20Object%20Reference) (OtherActor :type Actor%20Object%20Reference) (OtherComp :type Primitive%20Component%20Object%20Reference) (OtherBodyIndex :type Integer))
  ;[1 1 1] Slow Player In Water
  (Utilities|IsValid (Utilities|Array|Get(acopy) (Collision|GetOverlappingActors (Variables|Default|GetWaterSlow) "/Game/Blueprints/FirstPersonTemplate/BP_FirstPersonCharacter.BP_FirstPersonCharacter_C" :!class /Script/Engine.PrimitiveComponent))
    (:Is%20Not%20Valid
      (Development|PrintString "EndSlow")
      (bind _asbp_first_person_character (Utilities|Casting|CastToBP_FirstPersonCharacter OtherActor)
        (:then
          (bind _output_get (Variables|Default|SetPlayerCharacter _asbp_first_person_character))
          (Default|ReverseSlowPlayer _output_get))
        (:CastFailed
          (Development|PrintString "CastFailed"))))))

(event OnComponentBeginOverlap(WaterSlow)
  (params (OverlappedComponent :type Primitive%20Component%20Object%20Reference) (OtherActor :type Actor%20Object%20Reference) (OtherComp :type Primitive%20Component%20Object%20Reference) (OtherBodyIndex :type Integer) (bFromSweep :type Boolean) (SweepResult :type Hit%20Result%20Structure%20%28by%20ref%29))
  ;[1 1 1] Slow Player In Water
  (Utilities|IsValid (Utilities|Array|Get(acopy) (Collision|GetOverlappingActors (Variables|Default|GetWaterSlow) "/Game/Blueprints/FirstPersonTemplate/BP_FirstPersonCharacter.BP_FirstPersonCharacter_C" :!class /Script/Engine.PrimitiveComponent))
    (:Is%20Valid
      (if (Rendering|IsVisible (Variables|Default|GetSM_WaterPlain))
        (if (Rendering|IsVisible (Variables|Default|GetSM_WaterPlain1))
          (Development|PrintString "InWaterSlow")
          (bind _asbp_first_person_character (Utilities|Casting|CastToBP_FirstPersonCharacter OtherActor)
            (:then
              (bind _output_get (Variables|Default|SetPlayerCharacter _asbp_first_person_character))
              (Default|SlowPlayer _output_get))
            (:CastFailed
              (Development|PrintString "CastFailed"))))
        (else
          (Development|PrintString "NoWater"))))))

(fn ConstructionScript)