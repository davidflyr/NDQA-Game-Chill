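; FPS-Controller is a player controller Blueprint that feeds movement and look input to the first-person character.
; On BeginPlay it casts player character 0 to FPS-Character and caches it as PlayerRef.
; Each horizontal and vertical Move and Look axis event forwards its value to the character's Move or Look function, zeroing the other axis, so the character does the actual handling.
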(event EventBeginPlay
  (bind _asfps_character (Utilities|Casting|CastToFPS-Character (Game|GetPlayerCharacter 0)))
  (Variables|Default|SetPlayerRef _asfps_character))

(event Input|AxisEvents|InputAxisMoveHorizontal
  (params (AxisValue :type Float%20%28single-precision%29))
  (Default|Move (Variables|Default|GetPlayerRef) AxisValue 0.0))

(event Input|AxisEvents|InputAxisMoveVertical
  (params (AxisValue :type Float%20%28single-precision%29))
  (Default|Move (Variables|Default|GetPlayerRef) 0.0 AxisValue))

(event Input|AxisEvents|InputAxisLookHorizontal
  (params (AxisValue :type Float%20%28single-precision%29))
  (Default|Look (Variables|Default|GetPlayerRef) AxisValue 0.0))

(event Input|AxisEvents|InputAxisLookVertical
  (params (AxisValue :type Float%20%28single-precision%29))
  (Default|Look (Variables|Default|GetPlayerRef) 0.0 AxisValue))

(fn ConstructionScript)