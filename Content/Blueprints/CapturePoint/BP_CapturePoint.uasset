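; Capture point actor that the first-person player takes by standing inside its Box until progress reaches the CapturePoint threshold, then destroys itself.
; Delay-driven loops step progress up while the player holds it, pause it while AI enemies in EnemyCheck contest it, and drain it when enemies stand alone.
; The ProgressBar widget, taken from a widget component rotated on Tick using the player's position, is also shown in the viewport during capture.
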(event OnComponentEndOverlap(Box)
  (params (OverlappedComponent :type Primitive%20Component%20Object%20Reference) (OtherActor :type Actor%20Object%20Reference) (OtherComp :type Primitive%20Component%20Object%20Reference) (OtherBodyIndex :type Integer))
  ;[1 1 1] IsPlayerOFFPoint
  (Utilities|IsValid (Utilities|Array|Get(acopy) (Collision|GetOverlappingActors (Variables|Default|GetBox) "/Game/Blueprints/FirstPersonTemplate/BP_FirstPersonCharacter.BP_FirstPersonCharacter_C" :!class /Script/Engine.PrimitiveComponent))
    (:Is%20Not%20Valid
      (Utilities|Casting|CastToBP_FirstPersonCharacter OtherActor)
      (Variables|Default|SetPlayerOnPoint false)
      (Development|PrintString "OffPoint" false true "(R=0.000000,G=0.660000,B=1.000000,A=1.000000)" 5.0)
      (Widget|RemovefromParent (Variables|Default|GetProgressBar))
      (Variables|Default|SetProgressOnScreen false))))

(event OnComponentBeginOverlap(Box)
  (params (OverlappedComponent :type Primitive%20Component%20Object%20Reference) (OtherActor :type Actor%20Object%20Reference) (OtherComp :type Primitive%20Component%20Object%20Reference) (OtherBodyIndex :type Integer) (bFromSweep :type Boolean) (SweepResult :type Hit%20Result%20Structure%20%28by%20ref%29))
  ;[1 1 1] IsPlayerOnPoint
  (Utilities|IsValid (Utilities|Array|Get(acopy) (Collision|GetOverlappingActors (Variables|Default|GetBox) "/Game/Blueprints/FirstPersonTemplate/BP_FirstPersonCharacter.BP_FirstPersonCharacter_C" :!class /Script/Engine.PrimitiveComponent))
    (:Is%20Valid
      (Utilities|Casting|CastToBP_FirstPersonCharacter OtherActor)
      (Variables|Default|SetPlayerOnPoint true)
      (if (Variables|Default|GetPointTaken) :!label _label
        (Variables|Default|SetTakingPoint false)
        (else
          (Variables|Default|SetTakingPoint true)))
      (if (Variables|Default|GetTakingPoint)
        (Utilities|FlowControl|Delay 0.1)
        (Development|PrintString "TakingPoint" false true "(R=0.000000,G=0.660000,B=1.000000,A=1.000000)" 5.0)
        ;[1 1 1] AddProgressBarToPlayerScreen
        (if (Variables|Default|GetProgressOnScreen)
          _
          (else
            (UserInterface|Viewport|AddtoViewport (Variables|Default|GetProgressBar) 0)
            (Variables|Default|SetProgressOnScreen true)))
        ;[1 1 1] AddProgress
        (bind _output_get (Variables|Default|SetProgress (Math|Integer|Clamp(Integer) (+ (Variables|Default|GetProgress) 10) 0 100)))
        (Default|UpdateProgress (Variables|Default|GetProgressBar) _output_get)
        (Utilities|FlowControl|Delay 1.0)
        (if (>= (Variables|Default|GetProgress) (Variables|Default|GetCapturePoint))
          ;[1 1 1] Remove Capture Point From Scene
          (Variables|Default|SetPointTaken true)
          (Development|PrintString "PointCaptured" true true "(R=0.133611,G=1.000000,B=0.118760,A=1.000000)" 2e+01)
          (Actor|DestroyActor)
          (Widget|RemovefromParent (Variables|Default|GetProgressBar))
          (elif (Variables|Default|GetPlayerOnPoint)
            (if (not (Variables|Default|GetEnemyOnPoint))
              (goto _label))))
        (else
          (Utilities|FlowControl|Delay 0.1)
          (Development|PrintString "PointAlreadyTaken" false true "(R=0.180784,G=1.000000,B=0.336319,A=1.000000)" 1e+01))))))

(event OnComponentBeginOverlap(EnemyCheck)
  (params (OverlappedComponent :type Primitive%20Component%20Object%20Reference) (OtherActor :type Actor%20Object%20Reference) (OtherComp :type Primitive%20Component%20Object%20Reference) (OtherBodyIndex :type Integer) (bFromSweep :type Boolean) (SweepResult :type Hit%20Result%20Structure%20%28by%20ref%29))
  ;[1 1 1] IsEnemyOnPoint
  (Utilities|IsValid (Utilities|Array|Get(acopy) (Collision|GetOverlappingActors (Variables|Default|GetEnemyCheck) "/Game/ThirdPersonBP/Blueprints/AI_ThirdPersonCharacter.AI_ThirdPersonCharacter_C" :!class /Script/Engine.PrimitiveComponent)) :!label _label
    (:Is%20Valid
      (Utilities|Casting|CastToAI_ThirdPersonCharacter OtherActor)
      (if (Variables|Default|GetPlayerOnPoint)
        (Utilities|FlowControl|Delay 0.1)
        (Development|PrintString "NoProgress" false true "(R=1.000000,G=0.765628,B=0.062500,A=1.000000)" 5.0)
        (Utilities|IsValid (Utilities|Array|Get(acopy) (Collision|GetOverlappingActors (Variables|Default|GetEnemyCheck) "/Game/ThirdPersonBP/Blueprints/AI_ThirdPersonCharacter.AI_ThirdPersonCharacter_C" :!class /Script/Engine.PrimitiveComponent))
          (:Is%20Valid
            (Variables|Default|SetEnemyOnPoint true)
            (goto _label))
          (:Is%20Not%20Valid
            (Variables|Default|SetEnemyOnPoint false)
            ;[1 1 1] AddProgress
            (bind _output_get (Variables|Default|SetProgress (Math|Integer|Clamp(Integer) (+ (Variables|Default|GetProgress) 10) 0 100) :!label _label_2))
            (Default|UpdateProgress (Variables|Default|GetProgressBar) _output_get)
            (Utilities|FlowControl|Delay 1.0)
            (if (>= (Variables|Default|GetProgress) (Variables|Default|GetCapturePoint))
              ;[1 1 1] Remove Capture Point From Scene
              (Variables|Default|SetPointTaken true)
              (Development|PrintString "PointCaptured" true true "(R=0.133611,G=1.000000,B=0.118760,A=1.000000)" 2e+01)
              (Actor|DestroyActor)
              (Widget|RemovefromParent (Variables|Default|GetProgressBar))
              (elif (Variables|Default|GetPlayerOnPoint)
                (if (not (Variables|Default|GetEnemyOnPoint))
                  ;[1 1 1] IsPlayerOnPoint
                  (if (Variables|Default|GetPointTaken)
                    (Variables|Default|SetTakingPoint false)
                    (else
                      (Variables|Default|SetTakingPoint true)))
                  (if (Variables|Default|GetTakingPoint)
                    (Utilities|FlowControl|Delay 0.1)
                    (Development|PrintString "TakingPoint" false true "(R=0.000000,G=0.660000,B=1.000000,A=1.000000)" 5.0)
                    ;[1 1 1] AddProgressBarToPlayerScreen
                    (if (Variables|Default|GetProgressOnScreen)
                      (goto _label_2)
                      (else
                        (UserInterface|Viewport|AddtoViewport (Variables|Default|GetProgressBar) 0)
                        (Variables|Default|SetProgressOnScreen true)
                        (goto _label_2)))
                    (else
                      (Utilities|FlowControl|Delay 0.1)
                      (Development|PrintString "PointAlreadyTaken" false true "(R=0.180784,G=1.000000,B=0.336319,A=1.000000)" 1e+01))))))))
        (else
          (Utilities|FlowControl|Delay 0.1)
          (Development|PrintString "EnemyOnPoint" false)
          (bind _output_get_2 (Variables|Default|SetProgress (Math|Integer|Clamp(Integer) (- (Variables|Default|GetProgress) 10) 0 100)))
          (Default|UpdateProgress (Variables|Default|GetProgressBar) _output_get_2)
          (Utilities|FlowControl|Delay 1.0)
          (goto _label))))))

(event EventBeginPlay
  ;[1 1 1] Spawn Progress Bar
  (bind _asprogress_bar (Utilities|Casting|CastToProgressBar (UserInterface|GetUserWidgetObject (Variables|Default|GetProgress_Widget))))
  (Variables|Default|SetProgressBar _asprogress_bar))

(event EventTick
  (params (DeltaSeconds :type Float%20%28single-precision%29))
  (bind _progress_widget (Variables|Default|GetProgress_Widget))
  ;[1 1 1] Rotate Progress Bar
  (Transformation|SetWorldRotation _progress_widget (Math|Rotator|FindLookatRotation (Transformation|GetActorLocation (Game|GetPlayerCharacter 0)) (Transformation|GetWorldLocation _progress_widget)) false false))

(fn ConstructionScript)